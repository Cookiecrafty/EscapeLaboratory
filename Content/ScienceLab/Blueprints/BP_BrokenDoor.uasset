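; BP_BrokenDoor is a science lab double sliding door that opens while a BP_Body actor is inside its collision volume.
; Begin overlap plays a timeline that slides the two door meshes apart along local Y in opposite directions.
; End overlap reverses the same timeline to close them, with no count of how many bodies remain inside.
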(event `self.Collision.OnComponentBeginOverlap`
  (params (OverlappedComponent :type "PrimitiveComponent Object Reference") (OtherActor :type "Actor Object Reference") (OtherComp :type "PrimitiveComponent Object Reference") (OtherBodyIndex :type Integer) (bFromSweep :type Boolean) (SweepResult :type "HitResult Structure (by ref)"))
  ;[0 0.3281 0] SecurityBreach0X00CF52
  (cast `/Game/EurileneGene/Core/BP_Body` OtherActor)
  (bind (_direction _openandclosedoor) (`Timeline|Timeline` :!label _label)
    (:`Update`
      (bind _returnvalue (* _openandclosedoor 90.0))
      (`SceneComponent.K2_SetRelativeLocation` (`self.LabDoor03B`) (`KismetMathLibrary.MakeVector` 0.0 _returnvalue) false false)
      (`SceneComponent.K2_SetRelativeLocation` (`self.LabDoor03A`) (`KismetMathLibrary.MakeVector` 0.0 (* _returnvalue -1.0)) false false))))

(event `self.Collision.OnComponentEndOverlap`
  (params (OverlappedComponent :type "PrimitiveComponent Object Reference") (OtherActor :type "Actor Object Reference") (OtherComp :type "PrimitiveComponent Object Reference") (OtherBodyIndex :type Integer))
  ;[0 0.3281 0] SecurityBreach0X00CF52
  (cast `/Game/EurileneGene/Core/BP_Body` OtherActor)
  (goto _label :!via `Reverse`))

(fn `UserConstructionScript`)