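; BP_LabDoor01 is an automatic sliding lab door with a construction-time choice between two meshes.
; A BP_Body entering the collision plays a timeline that slides the mesh along local Y; leaving reverses it.
; Entry first calls EOT on the body's AC_0X00A21E component, if present.
; It also overwrites the player camera's post-process settings, with the PP_EndOfTransmission blendable at zero weight.
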(event `self.Collision.OnComponentEndOverlap`
  (params (OverlappedComponent :type "PrimitiveComponent Object Reference") (OtherActor :type "Actor Object Reference") (OtherComp :type "PrimitiveComponent Object Reference") (OtherBodyIndex :type Integer))
  ;[0 0.3281 0] AutoOpenAndColseDoor
  (cast `/Game/EurileneGene/Core/BP_Body` OtherActor)
  (bind (_direction _openandclosedoor) (`Timeline|Timeline` :!via `Reverse` :!label _label)
    (:`Update`
      (`SceneComponent.K2_SetRelativeLocation` (`self.LabDoor01`) (`KismetMathLibrary.MakeVector` 0.0 (* _openandclosedoor 105.0)) false false))))

(event `self.Collision.OnComponentBeginOverlap`
  (params (OverlappedComponent :type "PrimitiveComponent Object Reference") (OtherActor :type "Actor Object Reference") (OtherComp :type "PrimitiveComponent Object Reference") (OtherBodyIndex :type Integer) (bFromSweep :type Boolean) (SweepResult :type "HitResult Structure (by ref)"))
  ;[1 0 0] FatalCodeDoor42
  (bind _asbp_body (cast `/Game/EurileneGene/Core/BP_Body` OtherActor))
  (`|ExecutionSequence`
    (:`then_0`
      (bind _returnvalue (`self.GetComponentByClass` _asbp_body "/Game/ScienceLab/SecuritySystem/AC_0X00A21E.AC_0X00A21E_C"))
      (`/Engine/EditorBlueprintResources/StandardMacros.IsValid` _returnvalue
        (:`Is Valid`
          (`/Game/ScienceLab/SecuritySystem/AC_0X00A21E.EOT` _returnvalue))))
    (:`then_1`
      ;[0 0.3281 0] AutoOpenAndColseDoor
      (bind _asbp_body_2 (cast `/Game/EurileneGene/Core/BP_Body` (`GameplayStatics.GetPlayerPawn` 0)))
      (set `CameraComponent.PostProcessSettings` (make `PostProcessSettings` :`WeightedBlendables` (make `WeightedBlendables` (`|MakeArray` (make `WeightedBlendable` 0.0 "/Game/ScienceLab/SecuritySystem/PP_EndOfTransmission.PP_EndOfTransmission") :!type "WeightedBlendable Structure"))) (`/Game/EurileneGene/Core/BP_Body.FirstPersonCamera` _asbp_body_2))
      (goto _label))))

(fn `UserConstructionScript`
  (bind _labdoor01 (`self.LabDoor01`))
  ;[1 1 1] Change Door Mesh
  (switch `int` (`self.Door Mesh`)
    (:`Default`
      (`StaticMeshComponent.SetStaticMesh` _labdoor01 "/Game/ScienceLab/Meshes/Rooms/Doors/SM_LabDoor01.SM_LabDoor01" :!label _label))
    (:`0`
      (goto _label))
    (:`1`
      (`StaticMeshComponent.SetStaticMesh` _labdoor01 "/Game/ScienceLab/Meshes/Rooms/Doors/SM_LabDoor04.SM_LabDoor04"))))