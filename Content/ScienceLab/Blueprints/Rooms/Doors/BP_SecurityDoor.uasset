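; BP_SecurityDoor is a sliding double door in the science lab that opens only for authorized user IDs.
; CheckID looks up the ID's access level in DT_Users: Scientist, Manager and Headchief get a success sound and play the door timeline, while Visitors and unknown IDs get a failure sound.
; The timeline slides both panels apart in opposite directions, and reverses to close them when a BP_Body leaves the collision volume.
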(event `self.Collision.OnComponentEndOverlap`
  (params (OverlappedComponent :type "PrimitiveComponent Object Reference") (OtherActor :type "Actor Object Reference") (OtherComp :type "PrimitiveComponent Object Reference") (OtherBodyIndex :type Integer))
  ;[0 0.3281 0] AutoOpenAndColseDoor
  (cast `/Game/EurileneGene/Core/BP_Body` OtherActor)
  (bind (_direction _openandclosedoor) (`Timeline|Timeline` :!via `Reverse` :!label _label)
    (:`Update`
      (bind _returnvalue (* _openandclosedoor 90.0))
      (`SceneComponent.K2_SetRelativeLocation` (`self.DoorL`) (`KismetMathLibrary.MakeVector` 0.0 _returnvalue) false false)
      (`SceneComponent.K2_SetRelativeLocation` (`self.DoorR`) (`KismetMathLibrary.MakeVector` 0.0 (* _returnvalue -1.0)) false false))))

(event `/Game/ScienceLab/SecuritySystem/BPI_Identity.CheckID`
  (params (ID :type Name))
  ;[1 0 0] CheckSecurityAccess
  (bind _returnvalue (`|GetDataTableRow` "/Game/ScienceLab/SecuritySystem/DT_users.DT_Users" ID)
    (:`then`
      (switch `/Game/ScienceLab/SecuritySystem/Enum_Access` (`.Access_9_4F0B8EFD4FCC75DB3F278CB2C7274093` (break `/Game/ScienceLab/SecuritySystem/Struct_Employee` _returnvalue))
        (:`NewEnumerator0`
          _)
        (:`NewEnumerator1`
          (`GameplayStatics.PlaySound2D` "/Engine/EditorSounds/Notifications/CompileSuccess_Cue.CompileSuccess_Cue" 1.0 1.0 0.0 null null :!label _label_2)
          (goto _label))
        (:`NewEnumerator3`
          (goto _label_2))
        (:`NewEnumerator2`
          (goto _label_2))))
    (:`RowNotFound`
      _))
  (`GameplayStatics.PlaySound2D` "/Engine/EditorSounds/Notifications/CompileFailed_Cue.CompileFailed_Cue" 1.0 1.0 0.0 null null))

(fn `UserConstructionScript`)